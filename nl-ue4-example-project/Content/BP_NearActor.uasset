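; BP_NearActor is an actor that sets up a NEAR blockchain wallet connection menu in the game.
; On BeginPlay it creates the BP_NearMenu widget, passes it the Wallet and adds it to the viewport.
; A credentials test chain saves and reloads wallet credentials, then prints the integration-server authorization.
; Its CreateCredentials trigger, targeting the NEAR testnet, is not wired to any event.
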(event `self.ReceiveBeginPlay`
  ;[1 1 1] Add connection widget
  (bind _returnvalue (`|CreateWidget` "/Game/BP_NearMenu.BP_NearMenu_C"))
  (set `/Game/BP_NearMenu.wallet` (`self.wallet`) _returnvalue)
  (`UserWidget.AddToViewport` _returnvalue 0))

(event `on credentials created`
  (bind _wallet (`self.wallet`))
  ;[1 1 1] Test credentials creation
  (`NearlinkerWalletComponent.SaveCredentials` _wallet (`self.File Path`) (`self.Password`))
  (`NearlinkerWalletComponent.LoadCredentials` _wallet (`self.File Path`) (`self.Password`))
  (bind _returnvalue (`NearlinkerWalletComponent.GetAuthorizationForIntegrationServer` _wallet))
  (`KismetSystemLibrary.PrintString` _returnvalue))

(fn `UserConstructionScript`)